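; Blueprint function library whose GetAllTilesInRange returns the BP_HexTile tiles within a step range of a start tile or location.
; Without a valid start tile, it scans all hex tiles for a matching Loc, then expands outward ring by ring through AdjacentTiles.
; With PathFindGoThrough set, occupied tiles are included but not expanded past.
; It optionally removes the start tile and outputs tiles, grid Locs and world locations.
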(fn `GetAllTilesInRange`
  (params (RangeToCheck :type Integer) (`Starting Loc` :type "Vector2D Structure") (`StartingTile (Optional)` :type "/Game/Arrandor/Core/Blueprints/Tiles/BP_HexTile Object Reference") (`PathFind || Go Through` :type Boolean) (`Include Starting Point in Return` :type Boolean))
  (returns (Return :type "Array of /Game/Arrandor/Core/Blueprints/Tiles/BP_HexTile Object Reference") (`Return (Locs)` :type "Array of Vector2D Structure") (`Return (WorldLoc)` :type "Array of Vector Structure"))
  (locals (AllTiles :type "Array of /Game/Arrandor/Core/Blueprints/Tiles/BP_HexTile Object Reference") (PF :type Boolean) (SL :type "Vector2D Structure") (Range :type Integer) (ST :type "/Game/Arrandor/Core/Blueprints/Tiles/BP_HexTile Object Reference") (TilesToCheck :type "Array of /Game/Arrandor/Core/Blueprints/Tiles/BP_HexTile Object Reference") (ReturnArray :type "Array of /Game/Arrandor/Core/Blueprints/Tiles/BP_HexTile Object Reference") (CheckingArray :type "Array of /Game/Arrandor/Core/Blueprints/Tiles/BP_HexTile Object Reference") (ReturnLocs :type "Array of Vector2D Structure") (ReturnWLoc :type "Array of Vector Structure") (ISR :type Boolean))
  (bind _adjacenttiles (`/Game/Arrandor/Core/Blueprints/Tiles/BP_HexTile.AdjacentTiles` (`local.ST`)))
  (set `local.Range` RangeToCheck)
  (set `local.SL` `Starting Loc`)
  (set `local.PF` `PathFind || Go Through`)
  (set `local.ISR` `Include Starting Point in Return`)
  (`/Engine/EditorBlueprintResources/StandardMacros.IsValid` `StartingTile (Optional)`
    (:`Is Valid`
      (set `local.ST` `StartingTile (Optional)`))
    (:`Is Not Valid`
      (bind _outactors (`GameplayStatics.GetAllActorsOfClass` null "/Game/Arrandor/Core/Blueprints/Tiles/BP_HexTile.BP_HexTile_C"))
      (bind _output_get (set `local.AllTiles` _outactors))
      (for _array_element _output_get
        (if (`KismetMathLibrary.EqualExactly_Vector2DVector2D` (`/Game/Arrandor/Core/Blueprints/Tiles/BP_HexTile.Loc` _array_element) (`local.SL`))
          (set `local.ST` _array_element)
          (break)))))
  (set `local.TilesToCheck` _adjacenttiles)
  (set `local.CheckingArray` _adjacenttiles)
  (set `local.CheckingArray` (`local.TilesToCheck`) :!label _label)
  (`KismetArrayLibrary.Array_Clear` (`local.TilesToCheck`))
  (for _array_element_2 (`local.CheckingArray`)
    (if (`/Game/Arrandor/Core/Blueprints/Tiles/BP_HexTile.UnitHere` _array_element_2)
      (if (`local.PF`)
        (`KismetArrayLibrary.Array_AddUnique` (`local.ReturnArray`) _array_element_2)
        (else
          (`KismetArrayLibrary.Array_AddUnique` (`local.ReturnArray`) _array_element_2 :!label _label_2)
          (`KismetArrayLibrary.Array_Append` (`local.TilesToCheck`) (`/Game/Arrandor/Core/Blueprints/Tiles/BP_HexTile.AdjacentTiles` _array_element_2))))
      (else
        (goto _label_2))))
  (bind _result (`/Engine/EditorBlueprintResources/StandardMacros.DecrementInt` (`local.Range`))
    (:`  `
      (if (<= _result 0)
        (if (not (`local.ISR`))
          (`/Engine/EditorBlueprintResources/StandardMacros.IsValid` (`local.ST`)
            (:`Is Valid`
              (`KismetArrayLibrary.Array_RemoveItem` (`local.ReturnArray`) (`local.ST`)))
            (:`Is Not Valid`
              (for (_array_element_3 _array_index) (`local.ReturnArray`)
                (if (== (`/Game/Arrandor/Core/Blueprints/Tiles/BP_HexTile.Loc` _array_element_3) (`local.SL`))
                  (`KismetArrayLibrary.Array_Remove` (`local.ReturnArray`) _array_index)
                  (break))))))
        (`KismetArrayLibrary.Array_Clear` (`local.ReturnLocs`))
        (`KismetArrayLibrary.Array_Clear` (`local.ReturnWLoc`))
        (for _array_element_4 (`local.ReturnArray`)
          (`KismetArrayLibrary.Array_AddUnique` (`local.ReturnLocs`) (`/Game/Arrandor/Core/Blueprints/Tiles/BP_HexTile.Loc` _array_element_4))
          (`KismetArrayLibrary.Array_AddUnique` (`local.ReturnWLoc`) (`Actor.K2_GetActorLocation` _array_element_4)))
        (return (`local.ReturnArray`) (`local.ReturnLocs`) (`local.ReturnWLoc`))
        (else
          (goto _label))))))