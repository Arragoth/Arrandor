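; BP_ADPlayerPawn is a player-controlled camera pawn that pans over the grid and zooms with a spring arm.
; Movement axes step it along its forward and right vectors at Z zero, each clamping one world axis (X or Y) to BP_GridManager's GridBounds.
; Zoom input steps the arm length within ZoomBounds, and the reset action restores DefaultArmLength and StartingLocation.
; Movement looks up the grid manager on every axis event and applies no delta-time scaling.
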(event `InputAxis|Input_ForwardBack`
  (params (AxisValue :type "Float (single-precision)"))
  (bind (_returnvalue_x _returnvalue_y) (`KismetMathLibrary.BreakVector` (+ (* AxisValue (`self.MoveSpeed`) (`self.GetActorForwardVector`)) (`self.K2_GetActorLocation`))))
  (bind _outactors (`GameplayStatics.GetAllActorsOfClass` "/Game/Arrandor/Core/Blueprints/BP_GridManager.BP_GridManager_C"))
  (if (`KismetArrayLibrary.Array_IsValidIndex` _outactors)
    (bind _output (`|GetArrayItem` _outactors))
    (`/Engine/EditorBlueprintResources/StandardMacros.IsValid` _output
      (:`Is Valid`
        (bind _gridbounds_x (`KismetMathLibrary.BreakVector` (`/Game/Arrandor/Core/Blueprints/BP_GridManager.GridBounds` _output)))
        (`self.K2_SetActorLocation` (`KismetMathLibrary.MakeVector` (`KismetMathLibrary.FClamp` _returnvalue_x 0.0 _gridbounds_x) _returnvalue_y))))))

(event `InputAxis|Input_RightLeft`
  (params (AxisValue :type "Float (single-precision)"))
  (bind (_returnvalue_x _returnvalue_y) (`KismetMathLibrary.BreakVector` (+ (* AxisValue (`self.MoveSpeed`) (`self.GetActorRightVector`)) (`self.K2_GetActorLocation`))))
  (bind _outactors (`GameplayStatics.GetAllActorsOfClass` "/Game/Arrandor/Core/Blueprints/BP_GridManager.BP_GridManager_C"))
  (if (`KismetArrayLibrary.Array_IsValidIndex` _outactors)
    (bind _output (`|GetArrayItem` _outactors))
    (`/Engine/EditorBlueprintResources/StandardMacros.IsValid` _output
      (:`Is Valid`
        (bind (_gridbounds_x _gridbounds_y) (`KismetMathLibrary.BreakVector` (`/Game/Arrandor/Core/Blueprints/BP_GridManager.GridBounds` _output)))
        (`self.K2_SetActorLocation` (`KismetMathLibrary.MakeVector` _returnvalue_x (`KismetMathLibrary.FClamp` _returnvalue_y 0.0 _gridbounds_y)))))))

(event `InputAxis|Input_Zoom`
  (params (AxisValue :type "Float (single-precision)"))
  (bind (_zoombounds_x _zoombounds_y) (`KismetMathLibrary.BreakVector2D` (`self.ZoomBounds`)))
  (bind (_zoombounds_x_2 _zoombounds_y_2) (`KismetMathLibrary.BreakVector2D` (`self.ZoomBounds`)))
  (if (== AxisValue 0.0)
    _
    (elif (> AxisValue 0.0)
      (set `SpringArmComponent.TargetArmLength` (`KismetMathLibrary.FClamp` (- (`SpringArmComponent.TargetArmLength` (`self.SpringArm`)) (`self.ZoomSpeed`)) _zoombounds_x _zoombounds_y) (`self.SpringArm`))
      (else
        (set `SpringArmComponent.TargetArmLength` (`KismetMathLibrary.FClamp` (+ (`SpringArmComponent.TargetArmLength` (`self.SpringArm`)) (`self.ZoomSpeed`)) _zoombounds_x_2 _zoombounds_y_2) (`self.SpringArm`))))))

(event `InputAction|Input_ZoomReset`
  (params (Key :type "Key Structure"))
  (:`Pressed`
    (set `SpringArmComponent.TargetArmLength` (`self.Default Arm Length`) (`self.SpringArm`))
    (`self.K2_SetActorLocation` (`self.Starting Location`))))

(fn `UserConstructionScript`)