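; Game mode for a two-player turn-based match that seats joining players and alternates turns between them.
; PostLogin initializes each player's pawn, assigns player indices, has the controller find the grid manager, and starts the game when the second player joins.
; CycleTurns ends the active player's client turn, flips the turn index and starts the other's.
; ChoosePlayerStart looks up an index-keyed map of BP_ADPlayerStart actors using the player count.
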(event `self.K2_PostLogin`
  (params (NewPlayer :type "PlayerController Object Reference"))
  (bind _asbp_adplayer_controler (cast `/Game/Arrandor/Core/Blueprints/BP_ADPlayerControler` NewPlayer :!pure true))
  ;[1 1 1 1 17] Start Game when Two(2) Players join
  (`self.InitializePlayerPawn_Call` NewPlayer)
  (for (_array_element _array_index) (`GameStateBase.PlayerArray` (`GameplayStatics.GetGameState`))
    (bind _asbp_adplayer_state (cast `/Game/Arrandor/Core/Blueprints/BP_ADPlayerState` _array_element))
    (set `/Game/Arrandor/Core/Blueprints/BP_ADPlayerState.PlayerIndex` _array_index _asbp_adplayer_state))
  (bind _returnvalue (`self.GetNumPlayers`))
  (`/Game/Arrandor/Core/Blueprints/BP_ADPlayerControler.FindGridManager` _asbp_adplayer_controler)
  (bind _output_get (set `/Game/Arrandor/Core/Blueprints/BP_ADPlayerControler.PlayerIndex` (- _returnvalue 1) _asbp_adplayer_controler))
  (if (== _output_get 1)
    (`self.StartGame`)))

(event `StartGame`
  ;[1 1 1] Start Player Turn
  (`/Game/Arrandor/Core/Blueprints/BP_ADPlayerControler.StartTurn_Client` (`self.PlayerInTurn`)))

(event `CycleTurns`
  ;[1 1 1] Cycle Turns
  (`/Game/Arrandor/Core/Blueprints/BP_ADPlayerControler.EndTurn_Client` (`self.PlayerInTurn`))
  (set `self.CurrentPlayersTurn` (select `bool` (== (`self.CurrentPlayersTurn`) 0) :`true` 1))
  (`/Game/Arrandor/Core/Blueprints/BP_ADPlayerControler.StartTurn_Client` (`self.PlayerInTurn`)))

(fn `ChoosePlayerStart`
  (params (Player :type "Controller Object Reference"))
  (returns (ReturnValue :type "Actor Object Reference"))
  (`self.InitializeSpawnPoints`)
  (bind _returnvalue (`self.GetNumPlayers`))
  (return (`BlueprintMapLibrary.Map_Find` (`self.SpawnPoints`) _returnvalue)))

(fn `InitializePlayerPawn_Call`
  (params (Object :type "Object Object Reference"))
  (bind _asbp_adplayer_controler (cast `/Game/Arrandor/Core/Blueprints/BP_ADPlayerControler` Object))
  (`/Game/Arrandor/Core/Blueprints/BP_ADPlayerControler.InitializePlayerPawn` _asbp_adplayer_controler))

(fn `InitializeSpawnPoints`
  (if (== (`BlueprintMapLibrary.Map_Length` (`self.SpawnPoints`)) 0)
    (bind _outactors (`GameplayStatics.GetAllActorsOfClass` "/Game/Arrandor/Core/Blueprints/BP_ADPlayerStart.BP_ADPlayerStart_C"))
    (for _array_element _outactors
      (`BlueprintMapLibrary.Map_Add` (`self.SpawnPoints`) (`/Game/Arrandor/Core/Blueprints/BP_ADPlayerStart.GetPlayerIndex` _array_element) _array_element))))

(fn `UserConstructionScript`)