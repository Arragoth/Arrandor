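; Player controller for a turn-based, faction-based hex-grid tactics game that creates the player UI and tracks whose turn it is.
; Left-click release branches on ClickMode to select, spawn, move or attack with units, or swap faction tiles, reading the selected unit from W_PlayerUI.
; Request events run only on authority, forwarding to the game state, unit or grid manager.
; Aid and action ability checks are stubs returning false.
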(event `self.ReceiveBeginPlay`
  (if (`self.IsLocalController`)
    (bind _returnvalue (`|CreateWidget` "/Game/Arrandor/UI/W_PlayerUI.W_PlayerUI_C" self))
    (`UserWidget.AddToViewport` _returnvalue 0)))

(event `StartTurn_Client`
  (`self.SetMyTurn` true))

(event `FindGridManager`
  (`/Engine/EditorBlueprintResources/ActorMacros.Switch Has Authority`
    (:`Authority`
      (bind _outactors (`GameplayStatics.GetAllActorsOfClass` "/Game/Arrandor/Core/Blueprints/BP_GridManager.BP_GridManager_C"))
      (set `self.GameBoard` (`|GetArrayItem` _outactors)))))

(event `EndTurn_Client`
  (`self.SetMyTurn` false))

(event `InitializePlayerPawn`
  (`KismetSystemLibrary.PrintString` (`KismetSystemLibrary.GetDisplayName` (`self.K2_GetPawn`)) true true (struct :`G` 0.66 :`B` 1.0 :`A` 1.0) 30.0)
  (`/Engine/EditorBlueprintResources/ActorMacros.Switch Has Authority`
    (:`Authority`
      (`KismetSystemLibrary.PrintString` "auth" true true (struct :`G` 0.66 :`B` 1.0 :`A` 1.0) 30.0))
    (:`Remote`
      (`KismetSystemLibrary.PrintString` "remote" true true (struct :`G` 0.66 :`B` 1.0 :`A` 1.0) 30.0))))

(event `RequestSelectUnit`
  (params (Unit :type "/Game/Arrandor/Core/Blueprints/Units/BP_Unit Object Reference"))
  (`/Engine/EditorBlueprintResources/ActorMacros.Switch Has Authority`
    (:`Authority`
      (`/Game/Arrandor/Core/Blueprints/Units/BP_Unit.UnitSelected` Unit (`self.PlayerIndex`)))))

(event `Key|LeftMouseButton`
  (params (Key :type "Key Structure"))
  (bind (_bblockinghit _binitialoverlap _time _distance _location _impactpoint _normal _impactnormal _physmat _hitactor) (`GameplayStatics.BreakHitResult` (`self.GetHitResultUnderCursorByChannel` "TraceTypeQuery1")))
  (bind (_bblockinghit_2 _binitialoverlap_2 _time_2 _distance_2 _location_2 _impactpoint_2 _normal_2 _impactnormal_2 _physmat_2 _hitactor_2 _hitcomponent) (`GameplayStatics.BreakHitResult` (`self.GetHitResultUnderCursorByChannel` "TraceTypeQuery1")))
  (bind (_bblockinghit_3 _binitialoverlap_3 _time_3 _distance_3 _location_3 _impactpoint_3 _normal_3 _impactnormal_3 _physmat_3 _hitactor_3) (`GameplayStatics.BreakHitResult` (`self.GetHitResultUnderCursorByChannel` "TraceTypeQuery1")))
  (:`Released`
    (switch `/Game/Arrandor/Core/Enums/EN_ClickType` (`self.ClickMode`)
      (:`NewEnumerator0`
        (if _bblockinghit_3
          (bind _asbp_unit (cast `/Game/Arrandor/Core/Blueprints/Units/BP_Unit` _hitactor_3))
          (bind _foundwidgets (`WidgetBlueprintLibrary.GetAllWidgetsOfClass` "/Game/Arrandor/UI/W_PlayerUI.W_PlayerUI_C"))
          (`/Game/Arrandor/UI/W_PlayerUI.UnitSelect` (`|GetArrayItem` _foundwidgets) _asbp_unit)
          (`self.RequestSelectUnit` _asbp_unit)))
      (:`NewEnumerator1`
        (set `self.ClickMode` "NewEnumerator0")
        (if _bblockinghit_2
          (bind _asbp_hex_tile (cast `/Game/Arrandor/Core/Blueprints/Tiles/BP_HexTile` _hitactor_2))
          (if (not (`/Game/Arrandor/Core/Blueprints/Tiles/BP_HexTile.UnitHere` _asbp_hex_tile))
            (`self.Request Spawn Unit` "None" (`SceneComponent.K2_GetComponentLocation` _hitcomponent) (`/Game/Arrandor/Core/Blueprints/Tiles/BP_HexTile.Loc` _asbp_hex_tile) (`self.PlayerIndex`)))))
      (:`NewEnumerator2`
        (set `self.ClickMode` "NewEnumerator0")
        (if _bblockinghit
          (bind _asbp_hex_tile_2 (cast `/Game/Arrandor/Core/Blueprints/Tiles/BP_HexTile` _hitactor)
            (:`then`
              (if (not (`/Game/Arrandor/Core/Blueprints/Tiles/BP_HexTile.UnitHere` _asbp_hex_tile_2))
                (bind _output (`self.GetUI`)
                  (:`Is Valid`
                    (bind _selectedunit (`/Game/Arrandor/UI/W_PlayerUI.SelectedUnit` _output))
                    (if (not (`/Game/Arrandor/Core/Blueprints/Units/BP_Unit.bMoved` _selectedunit))
                      (`/Game/Arrandor/Core/Blueprints/Units/BP_Unit.DeSelect` _selectedunit)
                      (`AIBlueprintHelperLibrary.SimpleMoveToLocation` (`AIBlueprintHelperLibrary.GetAIController` _selectedunit) (`SceneComponent.K2_GetComponentLocation` (`/Game/Arrandor/Core/Blueprints/Tiles/BP_HexTile.StaticMesh` _asbp_hex_tile_2)))
                      (`self.RequestMoveUnit` _selectedunit _asbp_hex_tile_2)
                      (set `/Game/Arrandor/UI/W_PlayerUI.SelectedUnit` null _output))))))
            (:`CastFailed`
              (bind _asbp_unit_2 (cast `/Game/Arrandor/Core/Blueprints/Units/BP_Unit` _hitactor))
              (bind _output_2 (`self.GetUI`)
                (:`Is Valid`
                  (bind _selectedunit_2 (`/Game/Arrandor/UI/W_PlayerUI.SelectedUnit` _output_2))
                  (if (== _selectedunit_2 _asbp_unit_2)
                    (`/Game/Arrandor/Core/Blueprints/Units/BP_Unit.DeSelect` _selectedunit_2)
                    (set `/Game/Arrandor/UI/W_PlayerUI.SelectedUnit` null _output_2)
                    (else
                      ;[1 1 1] True = Aid || False = Attack
                      (if (== (`/Game/Arrandor/Core/Blueprints/Units/BP_Unit.OwnerIndex` _selectedunit_2) (`/Game/Arrandor/Core/Blueprints/Units/BP_Unit.OwnerIndex` _asbp_unit_2))
                        (bind _prompt (`self.CheckAidAbilities` _selectedunit_2 _asbp_unit_2))
                        (if _prompt
                          (bind _selectedunit_3 (`/Game/Arrandor/UI/W_PlayerUI.SelectedUnit` (stale _output_3)))
                          (`/Game/Arrandor/Core/Blueprints/Units/BP_Unit.DeSelect` _selectedunit_3 :!label _label)
                          (set `/Game/Arrandor/UI/W_PlayerUI.SelectedUnit` null (stale _output_3)))
                        (else
                          (bind _prompt_2 (`self.CheckActionAbilities` _selectedunit_2 _asbp_unit_2))
                          (bind _output_3 (`self.GetUI`)
                            (:`Is Valid`
                              (if _prompt_2
                                (goto _label)
                                (else
                                  (`self.RequestDealDamageToUnit` (`.Attack_20_AFD7E6414952A86F832F5EA56FCBE7BE` (break `/Game/Arrandor/Core/Struts/ST_Units` (`/Game/Arrandor/Core/Blueprints/Units/BP_Unit.Using_UnitInfo` _selectedunit_3))) _selectedunit_3 _asbp_unit_2)
                                  (goto _label)))))))))))))))
      (:`NewEnumerator3`
        (set `self.ClickMode` "NewEnumerator0")
        (bind _asbp_hex_tile_3 (cast `/Game/Arrandor/Core/Blueprints/Tiles/BP_HexTile` (`.HitActor` (`GameplayStatics.BreakHitResult` (`self.GetHitResultUnderCursorByChannel` "TraceTypeQuery1")))))
        (`self.ChangeFactionTile` _asbp_hex_tile_3)))))

(event `Request Spawn Unit`
  (params (RowName :type Name) (Location :type "Vector Structure") (Loc :type "Vector2D Structure") (OwnerIndex :type Integer))
  (`/Engine/EditorBlueprintResources/ActorMacros.Switch Has Authority`
    (:`Authority`
      (bind _asbp_adgame_state (cast `/Game/Arrandor/Core/Blueprints/BP_ADGAmeState` (`GameplayStatics.GetGameState`)))
      (`/Game/Arrandor/Core/Blueprints/BP_ADGAmeState.SpawnUnit_Server` _asbp_adgame_state RowName Location OwnerIndex Loc))))

(event `RequestMoveUnit`
  (params (UnitBeingMoved :type "/Game/Arrandor/Core/Blueprints/Units/BP_Unit Object Reference") (NewTile :type "/Game/Arrandor/Core/Blueprints/Tiles/BP_HexTile Object Reference"))
  (`/Engine/EditorBlueprintResources/ActorMacros.Switch Has Authority`
    (:`Authority`
      (bind _asbp_adgame_state (cast `/Game/Arrandor/Core/Blueprints/BP_ADGAmeState` (`GameplayStatics.GetGameState`)))
      (`/Game/Arrandor/Core/Blueprints/BP_ADGAmeState.UpdateTilesBeingMovedTo_Server` _asbp_adgame_state UnitBeingMoved NewTile))))

(event `AfterComfirm_UseActionAbility`
  (params (Caster :type "/Game/Arrandor/Core/Blueprints/Units/BP_Unit Object Reference") (Target :type "/Game/Arrandor/Core/Blueprints/Units/BP_Unit Object Reference")))

(event `RequestDealDamageToUnit`
  (params (`Raw Attack` :type Integer) (AttackingUnit :type "/Game/Arrandor/Core/Blueprints/Units/BP_Unit Object Reference") (TargetUnit :type "/Game/Arrandor/Core/Blueprints/Units/BP_Unit Object Reference"))
  (`/Engine/EditorBlueprintResources/ActorMacros.Switch Has Authority`
    (:`Authority`
      (bind _asbp_adgame_state (cast `/Game/Arrandor/Core/Blueprints/BP_ADGAmeState` (`GameplayStatics.GetGameState`)))
      (`/Game/Arrandor/Core/Blueprints/BP_ADGAmeState.DealDamageToUnit` _asbp_adgame_state AttackingUnit `Raw Attack` TargetUnit))))

(event `ChangeFactionTile`
  (params (CurrentTile :type "/Game/Arrandor/Core/Blueprints/Tiles/BP_HexTile Object Reference"))
  (`/Engine/EditorBlueprintResources/ActorMacros.Switch Has Authority`
    (:`Authority`
      (set `self.bTurnOptionDrawTile` false)
      (`/Game/Arrandor/Core/Blueprints/BP_GridManager.Click` (`self.GameBoard`) CurrentTile (select `/Game/Arrandor/Core/Enums/EN_Faction` (`self.PlayerFaction`) :`NewEnumerator0` "/Game/Arrandor/Core/Blueprints/Tiles/BP_HexTile_Solace.BP_HexTile_Solace_C" :`NewEnumerator1` "/Game/Arrandor/Core/Blueprints/Tiles/BP_HexTile_Corrupted.BP_HexTile_Corrupted_C" :!type "/Game/Arrandor/Core/Blueprints/Tiles/BP_HexTile Class Reference")))))

(fn `CheckActionAbilities`
  (params (`Casting Unit` :type "/Game/Arrandor/Core/Blueprints/Units/BP_Unit Object Reference") (`Target Unit` :type "/Game/Arrandor/Core/Blueprints/Units/BP_Unit Object Reference"))
  (returns (Prompt :type Boolean))
  (set `self.ActionAbilityHold_Index` "Test")
  (return false))

(fn `CheckAidAbilities`
  (params (`Casting Unit` :type "/Game/Arrandor/Core/Blueprints/Units/BP_Unit Object Reference") (`Target Unit` :type "/Game/Arrandor/Core/Blueprints/Units/BP_Unit Object Reference"))
  (returns (Prompt :type Boolean))
  (set `self.ActionAbilityHold_Index` "Test")
  (return false))

(fn `SetMyTurn`
  (params (MyTurn :type Boolean))
  (bind _output_get (set `self.bMyTurn?` MyTurn))
  (bind _output_get_2 (set `self.bTurnOptionDrawTile` _output_get))
  (`self.OnMyTurnChanged` _output_get_2))

(fn `UserConstructionScript`)