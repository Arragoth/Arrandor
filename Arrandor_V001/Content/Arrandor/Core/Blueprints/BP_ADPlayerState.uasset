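; Player state for Arrandor that handles a player's request to spawn a unit on the grid.
; RequestSpawnUnit traces under the given controller's cursor and, on a BP_GridManager hit, sets the controller's ClickMode.
; It then asks BP_ADGameState to spawn a hard-coded Skeleton at the hit component's location, owned by player state 0's PlayerIndex rather than its own.
; Debug prints trace the flow and failed game state cast.
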(event `RequestSpawnUnit`
  (params (PlayerController :type "/Game/Arrandor/Core/Blueprints/BP_ADPlayerControler Object Reference"))
  (bind _returnvalue (`GameplayStatics.GetGameState`))
  (bind (_bblockinghit _binitialoverlap _time _distance _location _impactpoint _normal _impactnormal _physmat _hitactor _hitcomponent) (`GameplayStatics.BreakHitResult` (`PlayerController.GetHitResultUnderCursorByChannel` PlayerController "TraceTypeQuery1" true)))
  (if _bblockinghit
    (cast `/Game/Arrandor/Core/Blueprints/BP_GridManager` _hitactor)
    (set `/Game/Arrandor/Core/Blueprints/BP_ADPlayerControler.ClickMode` "NewEnumerator0" PlayerController)
    (`KismetSystemLibrary.PrintString` "a" true true (struct :`G` 0.66 :`B` 1.0 :`A` 1.0) 30.0)
    (bind _asbp_adgame_state (cast `/Game/Arrandor/Core/Blueprints/BP_ADGameState` _returnvalue)
      (:`then`
        (`KismetSystemLibrary.PrintString` "b" true true (struct :`G` 0.66 :`B` 1.0 :`A` 1.0) 30.0)
        (`/Game/Arrandor/Core/Blueprints/BP_ADGameState.RequestSpawnUnit` _asbp_adgame_state "Skeleton" (`SceneComponent.K2_GetComponentLocation` _hitcomponent) (`/Game/Arrandor/Core/Blueprints/BP_ADPlayerState.PlayerIndex` (cast `/Game/Arrandor/Core/Blueprints/BP_ADPlayerState` (`GameplayStatics.GetPlayerState` 0) :!pure true))))
      (:`CastFailed`
        (`KismetSystemLibrary.PrintString` (`KismetSystemLibrary.GetDisplayName` _returnvalue) true true (struct :`G` 0.66 :`B` 1.0 :`A` 1.0) 30.0)))))

(fn `UserConstructionScript`)