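; Grid manager Blueprint that builds a hex tile map and lets individual tiles be changed.
; The construction script adds one static mesh component per cell, shifting odd X columns along Y by an offset to stagger the hexes.
; Tiles are stored in a map keyed by 2D grid index, and the overall grid bounds are saved.
; Click swaps a given tile's mesh and material.
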(fn `Click`
  (params (CurrentTile :type "StaticMeshComponent Object Reference") (NewTile :type "StaticMesh Object Reference") (NewMaterial :type "Material Object Reference"))
  (`StaticMeshComponent.SetStaticMesh` CurrentTile NewTile)
  (`PrimitiveComponent.SetMaterialByName` CurrentTile "None" NewMaterial))

(fn `UserConstructionScript`
  ;[1 1 1] Grid Creation
  (for _index (range (+ (`self.Grid_X`) 1))
    ;;[1 1 1] Calculates Size and Placement of of Grid Meshes
    (for _index_2 (range (+ (`self.Grid_Y`) 1))
      (bind _returnvalue (* _index (`self.Spacing X`)))
      (bind _returnvalue_2 (* _index_2 (`self.Spacing Y`)))
      ;;[1 1 1] Assign Mesh and Map Index of Grid Meshes
      (bind _returnvalue_3 (`AddComponent|NODE_AddStaticMeshComponent-0` :`RelativeTransform` (`KismetMathLibrary.MakeTransform` (`KismetMathLibrary.SelectVector` (`KismetMathLibrary.MakeVector` _returnvalue _returnvalue_2) (`KismetMathLibrary.MakeVector` _returnvalue (+ (`self.Offset`) _returnvalue_2)) (== (mod _index 2) 0)) (struct :`Yaw` 90.0))))
      (`BlueprintMapLibrary.Map_Add` (`self.HexTiles`) (`KismetMathLibrary.MakeVector2D` (`KismetMathLibrary.Conv_IntToDouble` _index) (`KismetMathLibrary.Conv_IntToDouble` _index_2)) _returnvalue_3)))
  (set `self.GridBounds` (`KismetMathLibrary.MakeVector` (* (`self.Grid_X`) (`self.Spacing X`)) (* (`self.Grid_Y`) (`self.Spacing Y`)))))